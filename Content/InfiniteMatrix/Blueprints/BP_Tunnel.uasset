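; BP_Tunnel is a tunnel segment in an endless runner with a continuously rolling obstacle wall.
; When the player enters its trigger box it asks the TunnelSpawner for a new segment and destroys itself, with end overlap adding score.
; Hitting the wall costs health and score, shakes the camera and can show restart, while an optional pack restores health.
; Functions randomize the hole mesh, its starting roll and the health pack's presence and position.
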(event OnComponentBeginOverlap(Box)
  (params (OverlappedComponent :type Primitive%20Component%20Object%20Reference) (OtherActor :type Actor%20Object%20Reference) (OtherComp :type Primitive%20Component%20Object%20Reference) (OtherBodyIndex :type Integer) (bFromSweep :type Boolean) (SweepResult :type Hit%20Result%20Structure%20%28by%20ref%29))
  ;[1 1 1] Tunnel Generation
  (Utilities|Casting|CastToBP_Player OtherActor)
  (Default|SpawnTunnelatSpawnPoint (Variables|Default|GetTunnelSpawner))
  (Actor|DestroyActor))

(event OnComponentBeginOverlap(WallMesh)
  (params (OverlappedComponent :type Primitive%20Component%20Object%20Reference) (OtherActor :type Actor%20Object%20Reference) (OtherComp :type Primitive%20Component%20Object%20Reference) (OtherBodyIndex :type Integer) (bFromSweep :type Boolean) (SweepResult :type Hit%20Result%20Structure%20%28by%20ref%29))
  ;[1 1 1] Obstacle Collision
  (bind _asbp_player (Utilities|Casting|CastToBP_Player OtherActor))
  (Default|ShakeCamera _asbp_player)
  (Default|UpdateTentativeScore _asbp_player -1e+01)
  (bind _isdead (Default|UpdateHealth _asbp_player -2e+01))
  (if _isdead
    (Default|DisplayRestart _asbp_player)))

(event OnComponentEndOverlap(Box)
  (params (OverlappedComponent :type Primitive%20Component%20Object%20Reference) (OtherActor :type Actor%20Object%20Reference) (OtherComp :type Primitive%20Component%20Object%20Reference) (OtherBodyIndex :type Integer))
  ;[1 1 1] Basic Score
  (bind _asbp_player (Utilities|Casting|CastToBP_Player OtherActor))
  (Default|UpdateScore _asbp_player 1e+01))

(event OnComponentBeginOverlap(HealthPackMesh)
  (params (OverlappedComponent :type Primitive%20Component%20Object%20Reference) (OtherActor :type Actor%20Object%20Reference) (OtherComp :type Primitive%20Component%20Object%20Reference) (OtherBodyIndex :type Integer) (bFromSweep :type Boolean) (SweepResult :type Hit%20Result%20Structure%20%28by%20ref%29))
  (bind _asbp_player (Utilities|Casting|CastToBP_Player OtherActor))
  (Default|UpdateHealth _asbp_player 2e+01)
  (Components|DestroyComponent (Variables|Default|GetHealthPackMesh)))

(event EventBeginPlay)

(event EventTick
  (params (DeltaSeconds :type Float%20%28single-precision%29))
  ;[1 1 1] Rotation
  (Transformation|AddLocalRotation (Variables|Default|GetWallMesh) (Math|Rotator|MakeRotator (* DeltaSeconds (Variables|Default|GetRotateSpeed)) 0.0 0.0) false false))

(fn ConstructionScript)

(fn RandomizeWall
  (Components|StaticMesh|SetStaticMesh (Variables|Default|GetWallMesh) (Utilities|Select :Index (Math|Random|RandomIntegerinRange 0 3) :Option%200 "/Game/InfiniteMatrix/Meshes/SM_Hole_01.SM_Hole_01" :Option%201 "/Game/InfiniteMatrix/Meshes/SM_Hole_02.SM_Hole_02" :Option%202 "/Game/InfiniteMatrix/Meshes/SM_Hole_03.SM_Hole_03" :Option%203 "/Game/InfiniteMatrix/Meshes/SM_Hole_04.SM_Hole_04"))
  (Transformation|AddLocalRotation (Variables|Default|GetWallMesh) (Math|Rotator|MakeRotator (Math|Random|RandomFloatinRange 0.0 3.6e+02) 0.0 0.0) false false))

(fn RandomizeHealthPack
  (bind (_x _y) (Utilities|RandomPolarCoordinate 3.6e+02))
  (bind _healthpackmesh (Variables|Default|GetHealthPackMesh))
  (Utilities|IsValid (Variables|Default|GetHealthPackMesh)
    (:Is%20Valid
      (if (< (Math|Random|RandomIntegerinRange 0 10) 3)
        (Transformation|AddWorldOffset _healthpackmesh (Math|Vector|MakeVector (Math|Random|RandomFloatinRange 1e+03 2.4e+03) _x _y) false false)
        (else
          (Components|DestroyComponent _healthpackmesh))))))
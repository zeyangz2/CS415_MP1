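; BP_Projectile is a player-linked projectile that ties its speed to the player and can award points.
; SetPlayer stores the Player reference that the other functions use.
; SetProjectileSpeed sets the ProjectileMovement max speed to a multiple of the player's ForwardSpeed, and IncreaseScore adds a fixed amount to the player's Score and refreshes its score text.
; The event graph is empty, so these functions run only when called from elsewhere.
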(event EventBeginPlay)

(event Collision|EventActorBeginOverlap
  (params (OtherActor :type Actor%20Object%20Reference)))

(event EventTick
  (params (DeltaSeconds :type Float%20%28single-precision%29)))

(fn ConstructionScript)

(fn SetProjectileSpeed
  (Variables|/Script/Engine.ProjectileMovementComponent|SetMaxSpeed (Variables|Default|GetProjectileMovement) (* (Variables|/Game/InfiniteMatrix/Blueprints/BP_Player.BP_Player_C|GetForwardSpeed (Variables|Default|GetPlayer)) 4.0)))

(fn SetPlayer
  (params (Player :type BP%20Player%20Object%20Reference))
  (Variables|Default|SetPlayer Player))

(fn IncreaseScore
  (bind _player (Variables|Default|GetPlayer))
  (Variables|/Game/InfiniteMatrix/Blueprints/BP_Player.BP_Player_C|SetScore _player (+ (Variables|/Game/InfiniteMatrix/Blueprints/BP_Player.BP_Player_C|GetScore _player) 20))
  (Default|UpdateScoreText _player))
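; BP_Enemy is a spinning hostile actor that damages the player on contact and awards score when shot.
; Tick rotates EnemyMesh around yaw at RotateSpeed, scaled by delta time.
; Overlapping BP_Player shakes its camera and subtracts health; a true result shows the restart display and destroys the enemy.
; Overlapping BP_Projectile destroys the projectile, adds score to the player pawn and destroys the enemy.
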(event EventBeginPlay)

(event Collision|EventActorBeginOverlap
  (params (OtherActor :type Actor%20Object%20Reference))
  (bind _asbp_player (Utilities|Casting|CastToBP_Player OtherActor)
    (:then
      (Default|ShakeCamera _asbp_player)
      (bind _isdead (Default|UpdateHealth _asbp_player -2e+01))
      (if _isdead
        (Default|DisplayRestart _asbp_player)
        (Actor|DestroyActor :!label _label)))
    (:CastFailed
      (bind _asbp_projectile (Utilities|Casting|CastToBP_Projectile OtherActor))
      (Actor|DestroyActor _asbp_projectile)
      (bind _asbp_player_2 (Utilities|Casting|CastToBP_Player (Game|Player|GetPlayerPawn 0)))
      (Default|UpdateScore _asbp_player_2 1e+01)
      (goto _label))))

(event EventTick
  (params (DeltaSeconds :type Float%20%28single-precision%29))
  (Transformation|AddLocalRotation (Variables|Default|GetEnemyMesh) (Math|Rotator|MakeRotator 0.0 0.0 (* DeltaSeconds (Variables|Default|GetRotateSpeed))) false false))

(fn ConstructionScript)